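; BP_Tile is one segment of an infinite terrain, populated with props and AI characters when play begins.
; BeginPlay locks the exit barrier and randomly scatters containers, rocks, other cover and AI pawns through PlaceActors and PlaceAIPawns.
; The player entering TileBounds swaps barrier collision and materials, opening the exit and sealing the entrance.
; Leaving asks InfiniteTerrainGameMode to spawn a tile, then destroys this one; an Arrow supplies the attach transform.
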(event `self.TileBounds.OnComponentEndOverlap`
  (params (OverlappedComponent :type "PrimitiveComponent Object Reference") (OtherActor :type "Actor Object Reference") (OtherComp :type "PrimitiveComponent Object Reference") (OtherBodyIndex :type Integer))
  (`self.Is Player Actor` OtherActor)
  (bind _asinfinite_terrain_game_mode (cast `/Game/Dynamic/InfiniteTerrainGameMode` (`GameplayStatics.GetGameMode`)))
  (`/Game/Dynamic/InfiniteTerrainGameMode.Spawn Tile` _asinfinite_terrain_game_mode)
  (`self.K2_DestroyActor`))

(event `self.TileBounds.OnComponentBeginOverlap`
  (params (OverlappedComponent :type "PrimitiveComponent Object Reference") (OtherActor :type "Actor Object Reference") (OtherComp :type "PrimitiveComponent Object Reference") (OtherBodyIndex :type Integer) (bFromSweep :type Boolean) (SweepResult :type "HitResult Structure (by ref)"))
  (`self.Is Player Actor` OtherActor)
  (`self.UnlockExit`))

(event `self.ReceiveBeginPlay`
  (`self.LockExit`)
  (`self.PlaceActors` "/Game/Dynamic/Terrain/Props/BP_Container.BP_Container_C" 1 5 400.0)
  (`self.PlaceActors` "/Game/Dynamic/Terrain/Props/BP_Box.BP_Box_C" 2 4 100.0 1.0 2.0)
  (`self.PlaceActors` "/Game/Dynamic/Terrain/Props/BP_Canister.BP_Canister_C" 1 7 50.0)
  (`self.PlaceActors` "/Game/Dynamic/Terrain/Props/BP_Rock01.BP_Rock01_C" 1 4 150.0 1.0 3.0)
  (`self.PlaceActors` "/Game/Dynamic/Terrain/Props/BP_Rock02.BP_Rock02_C" 1 4 250.0 1.0 3.0)
  (`self.PlaceActors` "/Game/Dynamic/Terrain/Props/BP_Rock03.BP_Rock03_C" 1 4 250.0 1.0 3.0)
  (`self.PlaceActors` "/Game/Dynamic/Terrain/Props/BP_SandBags.BP_SandBags_C" 1 2 250.0)
  (`self.PlaceAIPawns` "/Game/Dynamic/Character/Behavior/BP_Character.BP_Character_C" 2 4 100.0))

(fn `GetAttachLocation`
  (returns (AttachTransfrom :type "Transform Structure"))
  (return (`SceneComponent.K2_GetComponentToWorld` (`self.Arrow`))))

(fn `LockExit`
  (bind _exitbarrier (`self.ExitBarrier`))
  (bind _entrancebarrier (`self.EntranceBarrier`))
  (`PrimitiveComponent.SetCollisionEnabled` _exitbarrier "QueryAndPhysics")
  (`PrimitiveComponent.SetMaterial` _exitbarrier 0 "/Game/Dynamic/Terrain/MI_Red_Barrier.MI_Red_Barrier")
  (`PrimitiveComponent.SetCollisionEnabled` _entrancebarrier "NoCollision")
  (`PrimitiveComponent.SetMaterial` _entrancebarrier 0 "/Game/Dynamic/Terrain/MI_Transparent_Barrier.MI_Transparent_Barrier"))

(fn `UnlockEntrance`
  (bind _entrancebarrier (`self.EntranceBarrier`))
  (`PrimitiveComponent.SetCollisionEnabled` _entrancebarrier "NoCollision")
  (`PrimitiveComponent.SetMaterial` _entrancebarrier 0 "/Game/Dynamic/Terrain/MI_Transparent_Barrier.MI_Transparent_Barrier"))

(fn `UnlockExit`
  (bind _exitbarrier (`self.ExitBarrier`))
  (bind _entrancebarrier (`self.EntranceBarrier`))
  (`PrimitiveComponent.SetCollisionEnabled` _exitbarrier "NoCollision")
  (`PrimitiveComponent.SetMaterial` _exitbarrier 0 "/Game/Dynamic/Terrain/MI_Barrier_Green.MI_Barrier_Green")
  (`PrimitiveComponent.SetCollisionEnabled` _entrancebarrier "QueryAndPhysics")
  (`PrimitiveComponent.SetMaterial` _entrancebarrier 0 "/Game/Dynamic/Terrain/MI_Red_Barrier.MI_Red_Barrier"))

(fn `UserConstructionScript`)