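; Game mode for infinite terrain that spawns a chain of BP_Tile actors and keeps the score.
; On BeginPlay it populates a nav mesh bounds volume pool, then spawns the first few tiles.
; SpawnTile hands each tile the shared pool, unlocks its entrance and stores its attach location as the next spawn transform.
; NewTileConquered only increments Score.
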(event `self.ReceiveBeginPlay`
  (`self.PopulateBoundsVolumePool`)
  (for _ (range 3)
    (`self.Spawn Tile`)))

(fn `NewTileConquered`
  (bind _result (`/Engine/EditorBlueprintResources/StandardMacros.IncrementInt` (`self.Score`))
    (:`  `
      (set `self.Score` _result))))

(fn `Spawn Tile`
  (bind _returnvalue (`|SpawnActorFromClass` "/Game/Dynamic/Terrain/BP_Tile.BP_Tile_C" (`self.NextTileTransform`) "Undefined" "OverrideRootScale" null null))
  (`Tile.SetPool` _returnvalue (`self.NavMeshBoundsVolumePool`))
  (`/Game/Dynamic/Terrain/BP_Tile.UnlockEntrance` _returnvalue)
  (bind _attachtransfrom (`/Game/Dynamic/Terrain/BP_Tile.GetAttachLocation` _returnvalue))
  (set `self.NextTileTransform` _attachtransfrom))

(fn `UserConstructionScript`)